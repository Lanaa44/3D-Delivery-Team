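; Base station Blueprint that lets one character at a time perform an animated activity at it.
; StartInteraction walks the character by AI to an approach point, then onto the position marker, and snaps its rotation.
; It then plays paired station and character animations looked up by character class, releasing the character on montage completion or movement failure.
; The construction script derives both points' transforms from flattened position and facing vectors.
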(event `StartInteraction`
  (params (InteractingCharacter :type "/Game/Assets/Characters/NPC_Base Object Reference"))
  (bind _currentcharacter (`self.CurrentCharacter`))
  (bind _value (`BlueprintMapLibrary.Map_Find` (`self.StationAnimationsByClass`) (`self.CurrentCharClass`)))
  (`/Engine/EditorBlueprintResources/StandardMacros.IsValid` (`self.CurrentCharacter`)
    (:`Is Not Valid`
      (set `self.CurrentCharClass` (`GameplayStatics.GetObjectClass` InteractingCharacter))
      (bind _output_get (set `self.CurrentCharacter` InteractingCharacter))
      (`/Game/Assets/Characters/NPC_Base.StartInteracting` _output_get)
      ; Go to Activity Approach Start Point
      (`|AIMoveTo` _currentcharacter (`SceneComponent.K2_GetComponentLocation` (`self.ActivityApproachPoint`)) null
        (:`OnSuccess`
          ; Approach Activity Start Point
          (`|AIMoveTo` _currentcharacter (`SceneComponent.K2_GetComponentLocation` (`self.ActivityPositionMarker`)) null 0.5
            (:`OnSuccess`
              (`self.K2_SetActorRotation` (`self.CurrentCharacter`) (`SceneComponent.K2_GetComponentRotation` (`self.ActivityPositionMarker`)) false)
              ; Play Animations as Appropriate
              (`SkeletalMeshComponent.PlayAnimation` (`self.StationMesh`) (break `/Game/Assets/Stations/StationAnimations` _value) false)
              (`|PlayMontage` (`Character.Mesh` (`self.CurrentCharacter`)) (`.CharacterAnimation_5_BE30331E48454D942CD2AA95D8D7049C` (break `/Game/Assets/Stations/StationAnimations` _value))
                (:`OnCompleted`
                  _)))
            (:`OnFail`
              (`KismetSystemLibrary.PrintString` "Failed to reach start Point"))))
        (:`OnFail`
          _))
      (`/Game/Assets/Characters/NPC_Base.StopInteracting` (`self.CurrentCharacter`))
      (set `self.CurrentCharacter` null))))

(fn `UserConstructionScript`
  (bind _activitypositionmarker (`self.ActivityPositionMarker`))
  (bind (_activityposition_x _activityposition_y) (`KismetMathLibrary.BreakVector` (`self.ActivityPosition`)))
  (bind (_activityfacing_x _activityfacing_y) (`KismetMathLibrary.BreakVector` (`self.ActivityFacing`)))
  (bind _activityapproachpoint (`self.ActivityApproachPoint`))
  (bind _activityposition (`self.ActivityPosition`))
  (bind _returnvalue (`KismetMathLibrary.FindLookAtRotation` _activityposition (`self.ActivityFacing`)))
  (set `self.ActivityFacing` (`KismetMathLibrary.MakeVector` _activityfacing_x _activityfacing_y))
  (set `self.ActivityPosition` (`KismetMathLibrary.MakeVector` _activityposition_x _activityposition_y))
  (`SceneComponent.K2_SetRelativeLocation` _activitypositionmarker (+ (`self.ActivityPosition`) (0.0 0.0 0.1)) false false)
  (`SceneComponent.K2_SetRelativeRotation` _activitypositionmarker (`KismetMathLibrary.FindLookAtRotation` (`self.ActivityPosition`) (`self.ActivityFacing`)) false false)
  (`SceneComponent.K2_SetRelativeLocation` _activityapproachpoint (- _activityposition (`KismetMathLibrary.GreaterGreater_VectorRotator` (`KismetMathLibrary.MakeVector` (`self.ActivityApproachPointDistance`)) _returnvalue)) false false)
  (`SceneComponent.K2_SetRelativeRotation` _activityapproachpoint _returnvalue false false))