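; Building actor that toggles between exterior and interior views by swapping the mesh on a single static mesh component.
; On BeginPlay it caches the Template_PC player controller, then creates a BuildingHUD_W widget bound to itself and adds it to the viewport.
; ToggleBuilding flips ShowingInterior and sets the matching mesh, while the construction script applies the same choice in the editor.
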(event `self.ReceiveBeginPlay`
  (bind _astemplate_pc (cast `/Game/Core/Template_PC` (`GameplayStatics.GetPlayerController` 0)))
  (set `self.TemplatePC` _astemplate_pc)
  (bind _returnvalue (`|CreateWidget` "/Game/UI/BuildingHUD_W.BuildingHUD_W_C" null self))
  (bind _output_get (set `self.HUD` _returnvalue))
  (`UserWidget.AddToViewport` _output_get 0))

(event `ToggleBuilding`
  (bind _buildingexterior (`self.BuildingExterior`))
  (if (`self.ShowingInterior`)
    (set `self.ShowingInterior` false)
    (`StaticMeshComponent.SetStaticMesh` _buildingexterior (`self.ExteriorMesh`))
    (else
      (set `self.ShowingInterior` true)
      (`StaticMeshComponent.SetStaticMesh` _buildingexterior (`self.InteriorMesh`)))))

(fn `UserConstructionScript`
  (`StaticMeshComponent.SetStaticMesh` (`self.BuildingExterior`) (select `bool` (`self.ShowingInterior`) :`false` (`self.ExteriorMesh`) :`true` (`self.InteriorMesh`))))